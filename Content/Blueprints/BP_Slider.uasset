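; Slider actor whose mesh can be picked up, dragged along a slide axis, and coasts after release.
; Drag projects movement onto the axis and clamps the offset between slide limits; Drop takes the last offset change as speed.
; While released, Tick applies friction, reverses speed at half strength at MaxSlide, and floors the offset at zero.
; Construction caches the mesh's world transform, which serves as the base for relative-location updates.
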(event `self.ReceiveTick`
  (params (DeltaSeconds :type "Float (single-precision)"))
  (bind _speed (`self.Speed`))
  (bind _initialtransform_location (`KismetMathLibrary.BreakTransform` (`self.InitialTransform`)))
  (bind _returnvalue (* DeltaSeconds (`self.Friction`)))
  (if (`self.Held`)
    _
    (elif (> _speed 0.0)
      (bind _output_get (set `self.Speed` (- _speed _returnvalue)))
      (bind _returnvalue_2 (`KismetMathLibrary.FMax` (+ _output_get (`self.Offset`))))
      (if (>= _returnvalue_2 (`self.MaxSlide`)) :!label _label
        (set `self.Speed` (* (`self.Speed`) -0.5)))
      (bind _output_get_2 (set `self.Offset` _returnvalue_2))
      (`SceneComponent.K2_SetRelativeLocation` (`self.Mesh`) (+ _initialtransform_location (* (`self.SlideAxis`) _output_get_2)) false false)
      (elif (< _speed 0.0)
        (set `self.Speed` (+ _speed _returnvalue))
        (goto _label)))))

(event `/Game/Blueprints/PickupActorInterface.Pickup`
  (params (AttachTo :type "SceneComponent Object Reference"))
  (set `self.Held` true))

(event `/Game/Blueprints/PickupActorInterface.Drag`
  (params (Movement :type "Vector Structure"))
  (bind _offset (`self.Offset`))
  (bind _initialtransform_location (`KismetMathLibrary.BreakTransform` (`self.InitialTransform`)))
  (set `self.LastOffset` _offset)
  (bind _output_get (set `self.Offset` (`KismetMathLibrary.FClamp` (+ _offset (`KismetMathLibrary.Dot_VectorVector` Movement (`KismetMathLibrary.Normal` (`self.SlideAxis`)))) (`self.MinSlide`) (`self.MaxSlide`))))
  (`SceneComponent.K2_SetRelativeLocation` (`self.Mesh`) (+ _initialtransform_location (* (`self.SlideAxis`) _output_get)) false false))

(event `/Game/Blueprints/PickupActorInterface.Drop`
  (set `self.Held` false)
  (set `self.Speed` (- (`self.Offset`) (`self.LastOffset`))))

(fn `UserConstructionScript`
  (set `self.InitialTransform` (`SceneComponent.K2_GetComponentToWorld` (`self.Mesh`))))