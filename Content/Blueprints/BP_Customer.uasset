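; BP_Customer is a customer actor that gives itself a randomised face and colour tone.
; The construction script creates a dynamic material instance on FaceMesh, then calls RandomiseFeatures.
; That function picks random eye, nose and mouth textures for the face material and a random tone for the Mesh materials' Colour parameter.
; Any actor overlap re-rolls the look at runtime.
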(event `self.ReceiveActorBeginOverlap`
  (params (OtherActor :type "Actor Object Reference"))
  (`self.RandomiseFeatures`))

(fn `RandomiseFeatures`
  (bind _eyes (`self.Eyes`))
  (bind _tones (`self.Tones`))
  (bind _noses (`self.Noses`))
  (bind _mouthes (`self.Mouthes`))
  (`|ExecutionSequence`
    (:`then_0`
      (`MaterialInstanceDynamic.SetTextureParameterValue` (`self.FaceMaterial`) "EyeTexture" (`KismetArrayLibrary.Array_Get` _eyes (`KismetMathLibrary.RandomIntegerInRange` 0 (- (`KismetArrayLibrary.Array_Length` _eyes) 1)))))
    (:`then_1`
      (`MaterialInstanceDynamic.SetTextureParameterValue` (`self.FaceMaterial`) "NoseTexture" (`KismetArrayLibrary.Array_Get` _noses (`KismetMathLibrary.RandomIntegerInRange` 0 (- (`KismetArrayLibrary.Array_Length` _noses) 1)))))
    (:`then_2`
      (`MaterialInstanceDynamic.SetTextureParameterValue` (`self.FaceMaterial`) "MouthTexture" (`KismetArrayLibrary.Array_Get` _mouthes (`KismetMathLibrary.RandomIntegerInRange` 0 (- (`KismetArrayLibrary.Array_Length` _mouthes) 1)))))
    (:`then_3`
      (`MeshComponent.SetVectorParameterValueOnMaterials` (`self.Mesh`) "Colour" (`KismetMathLibrary.Conv_LinearColorToVector` (`KismetArrayLibrary.Array_Get` _tones (`KismetMathLibrary.RandomIntegerInRange` 0 (- (`KismetArrayLibrary.Array_Length` _tones) 1))))))))

(fn `UserConstructionScript`
  (bind _facemesh (`self.FaceMesh`))
  (bind _returnvalue (`PrimitiveComponent.CreateDynamicMaterialInstance` _facemesh 0 (`PrimitiveComponent.GetMaterial` _facemesh 0)))
  (bind _output_get (set `self.FaceMaterial` _returnvalue))
  (`PrimitiveComponent.SetMaterial` _facemesh 0 _output_get)
  (`self.RandomiseFeatures`))