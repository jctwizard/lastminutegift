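; BP_StickyMesh is a grabbable physics prop that can stick to other objects when dropped.
; The construction script applies one mesh reference to both the visible Mesh and the StickyCollider.
; Pickup disables physics and attaches the root to the supplied component, while Drag does nothing.
; Drop restores physics, detaches, then welds the root to the parent of the first overlapping component tagged "Sticky".
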(event `/Game/Blueprints/PickupActorInterface.Pickup`
  (params (AttachTo :type "SceneComponent Object Reference"))
  (`PrimitiveComponent.SetSimulatePhysics` (`self.Mesh`) false)
  (`SceneComponent.K2_AttachToComponent` (`self.K2_GetRootComponent`) AttachTo "None" "KeepWorld" "KeepWorld" "KeepWorld" false))

(event `/Game/Blueprints/PickupActorInterface.Drag`
  (params (Movement :type "Vector Structure")))

(event `/Game/Blueprints/PickupActorInterface.Drop`
  (`PrimitiveComponent.SetSimulatePhysics` (`self.Mesh`) true)
  (`self.K2_DetachFromActor` "KeepWorld" "KeepWorld" "KeepWorld")
  (for _array_element (`PrimitiveComponent.GetOverlappingComponents` (`self.StickyCollider`))
    (if (`ActorComponent.ComponentHasTag` _array_element "Sticky")
      (`SceneComponent.K2_AttachToComponent` (`self.K2_GetRootComponent`) (`KismetArrayLibrary.Array_Get` (`SceneComponent.GetParentComponents` _array_element)) "None" "KeepWorld" "KeepWorld" "KeepWorld" true)
      (break))))

(fn `UserConstructionScript`
  (`StaticMeshComponent.SetStaticMesh` (`self.Mesh`) (`self.MeshReference`))
  (`StaticMeshComponent.SetStaticMesh` (`self.StickyCollider`) (`self.MeshReference`)))