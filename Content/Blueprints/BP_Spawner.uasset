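; BP_Spawner is a grabbable mesh object that replenishes itself by leaving a fresh copy behind when first picked up.
; Construction applies MeshReference to Mesh and StickyCollider; BeginPlay disables physics and randomizes the material colour.
; It rotates every tick until grabbed.
; Pickup spawns a same-class replacement with the same mesh reference on first grab, then always disables physics and attaches itself to the given component, keeping world transform.
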(event `self.ReceiveBeginPlay`
  (bind _mesh (`self.Mesh`))
  (`PrimitiveComponent.SetSimulatePhysics` (`self.Mesh`) false)
  (`PrimitiveComponent.SetMaterial` _mesh 0 "/Game/Meshes/Customer_Mat.Customer_Mat")
  (`MeshComponent.SetVectorParameterValueOnMaterials` _mesh "Colour" (+ (* (`KismetMathLibrary.RandomUnitVector`) 0.5) (0.5 0.5 0.5))))

(event `self.ReceiveTick`
  (params (DeltaSeconds :type "Float (single-precision)"))
  (if (not (`self.Grabbed`))
    (`SceneComponent.K2_AddWorldRotation` (`self.Mesh`) (struct :`Pitch` 1.0 :`Roll` 1.0) false false)))

(event `/Game/Blueprints/PickupActorInterface.Pickup`
  (params (AttachTo :type "SceneComponent Object Reference"))
  (`|ExecutionSequence`
    (:`then_0`
      (if (not (`self.Grabbed`))
        (`|SpawnActorFromClass` (`GameplayStatics.GetObjectClass` self) (`self.GetTransform`) "Undefined" "OverrideRootScale" null (`self.MeshReference`))
        (set `self.Grabbed` true)))
    (:`then_1`
      (`PrimitiveComponent.SetSimulatePhysics` (`self.Mesh`) false)
      (`SceneComponent.K2_AttachToComponent` (`self.K2_GetRootComponent`) AttachTo "None" "KeepWorld" "KeepWorld" "KeepWorld" false))))

(fn `UserConstructionScript`
  (`StaticMeshComponent.SetStaticMesh` (`self.Mesh`) (`self.MeshReference`))
  (`StaticMeshComponent.SetStaticMesh` (`self.StickyCollider`) (`self.MeshReference`)))